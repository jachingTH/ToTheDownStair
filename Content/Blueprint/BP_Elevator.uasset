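; Elevator Blueprint that animates two sliding doors between their BeginPlay closed positions and a fixed open offset.
; OnInteract toggles the doors by playing or reversing the DoorAnimation timeline, whose finish flips the open state and calls OnDoorFinishedClosing in either direction.
; OpenDoor opens them through a separate timeline, blocked only while both animating and open.
; Both timelines lerp relative locations and maintain the animating flag exposed by IsCurrentlyAnimating.
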(event Custom|OpenDoor
  (if (not (and (Variables|Default|GetIsAnimating) (Variables|Default|GetIsDoorOpen)))
    (Variables|Default|SetIsAnimating true)
    (bind _alpha (Timeline|Timeline PlayFromStart)
      (:Update
        (Utilities|FlowControl|Sequence
          (:then_0
            (Transformation|SetRelativeLocation (Variables|Default|GetElevatorAnimation_Door1) (Math|Vector|Lerp(Vector) (Variables|Default|GetDoor1ClosePosition) (Variables|Default|GetDoor1OpenPosition) _alpha) false false))
          (:then_1
            (Transformation|SetRelativeLocation (Variables|Default|GetElevatorAnimation_Door2) (Math|Vector|Lerp(Vector) (Variables|Default|GetDoor2ClosePosition) (Variables|Default|GetDoor2OpenPosition) _alpha) false false))))
      (:Finished
        (Variables|Default|SetIsDoorOpen true)
        (Variables|Default|SetIsAnimating false)))))

(event EventBeginPlay
  (Variables|Default|SetDoor1ClosePosition (Variables|/Script/Engine.SceneComponent|GetRelativeLocation (Variables|Default|GetElevatorAnimation_Door1)))
  (Variables|Default|SetDoor2ClosePosition (Variables|/Script/Engine.SceneComponent|GetRelativeLocation (Variables|Default|GetElevatorAnimation_Door2)))
  (Variables|Default|SetDoor1OpenPosition "-200.000000,0.000000,0.000000")
  (Variables|Default|SetDoor2OpenPosition "-200.000000,0.000000,0.000000"))

(event EventOnInteract
  ;[1 1 1] Door Close
  (Variables|Default|SetIsAnimating true)
  (if (Variables|Default|GetIsDoorOpen)
    (bind _alpha (Timeline|DoorAnimation PlayFromStart)
      (:Update
        (Utilities|FlowControl|Sequence
          (:then_0
            (Transformation|SetRelativeLocation (Variables|Default|GetElevatorAnimation_Door1) (Math|Vector|Lerp(Vector) (Variables|Default|GetDoor1OpenPosition) (Variables|Default|GetDoor1ClosePosition) _alpha) false false))
          (:then_1
            (Transformation|SetRelativeLocation (Variables|Default|GetElevatorAnimation_Door2) (Math|Vector|Lerp(Vector) (Variables|Default|GetDoor2OpenPosition) (Variables|Default|GetDoor2ClosePosition) _alpha) false false))))
      (:Finished
        (Variables|Default|SetIsAnimating false)
        (Variables|Default|SetIsDoorOpen (not (Variables|Default|GetIsDoorOpen)))
        (Default|CallOnDoorFinishedClosing)))
    (else
      (Timeline|DoorAnimation ReverseFromEnd))))

(fn ConstructionScript)

(fn IsCurrentlyAnimating
  (return (Variables|Default|GetIsAnimating)))