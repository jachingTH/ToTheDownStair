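; BP_WindowBloodHand is an anomaly actor whose decals, presumably bloody handprints on a window, fade with player proximity.
; BeginPlay creates a dynamic material for each decal component.
; While armed by ActiveAnomaly, the box overlap plays a timeline driving Opacity_Alpha forward when the first-person character enters and in reverse on exit.
; ResetAnomaly disarms it and stops the timeline without resetting opacity.
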(event OnComponentBeginOverlap(Box)
  (params (OverlappedComponent :type Primitive%20Component%20Object%20Reference) (OtherActor :type Actor%20Object%20Reference) (OtherComp :type Primitive%20Component%20Object%20Reference) (OtherBodyIndex :type Integer) (bFromSweep :type Boolean) (SweepResult :type Hit%20Result%20Structure%20%28by%20ref%29))
  (if (Variables|Default|GetIsArmed)
    (Utilities|Casting|CastToBP_FirstPersonCharacter OtherActor)
    (bind _alpha (Timeline|FadeInAnimation PlayFromStart)
      (:Update
        (for _array_element (Variables|Default|GetDynamicDecalMaterials)
          (Rendering|Material|SetScalarParameterValue _array_element "Opacity_Alpha" _alpha :!class /Script/Engine.MaterialInstanceDynamic))))))

(event OnComponentEndOverlap(Box)
  (params (OverlappedComponent :type Primitive%20Component%20Object%20Reference) (OtherActor :type Actor%20Object%20Reference) (OtherComp :type Primitive%20Component%20Object%20Reference) (OtherBodyIndex :type Integer))
  (Utilities|Casting|CastToBP_FirstPersonCharacter OtherActor)
  (if (Variables|Default|GetIsArmed)
    (bind _alpha (Timeline|FadeInAnimation ReverseFromEnd)
      (:Update
        (for _array_element (Variables|Default|GetDynamicDecalMaterials)
          (Rendering|Material|SetScalarParameterValue _array_element "Opacity_Alpha" _alpha :!class /Script/Engine.MaterialInstanceDynamic))))))

(event EventActiveAnomaly
  (Variables|Default|SetIsArmed true))

(event EventResetAnomaly
  (Variables|Default|SetIsArmed false)
  (bind _alpha (Timeline|FadeInAnimation Stop)
    (:Update
      (for _array_element (Variables|Default|GetDynamicDecalMaterials)
        (Rendering|Material|SetScalarParameterValue _array_element "Opacity_Alpha" _alpha :!class /Script/Engine.MaterialInstanceDynamic)))))

(event EventBeginPlay
  (for _array_element (Actor|GetComponentsByClass "/Script/Engine.DecalComponent")
    (bind _returnvalue (Rendering|Material|CreateDynamicMaterialInstance _array_element :!class /Script/Engine.DecalComponent))
    (Utilities|Array|Add (Variables|Default|GetDynamicDecalMaterials) _returnvalue)))

(fn ConstructionScript)