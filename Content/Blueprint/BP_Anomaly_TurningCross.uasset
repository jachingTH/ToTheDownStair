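; BP_Anomaly_TurningCross is an anomaly actor whose cross rotates when the first-person player enters its collision volume while armed.
; ActiveAnomaly arms it, and the first qualifying overlap plays a timeline that lerps a pitch offset up to TargetRotationAngle, combined with the rotation cached at BeginPlay.
; A DoOnce limits this to one trigger until ResetAnomaly stops the timeline, restores the initial rotation, disarms it and reopens the gate.
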(event OnComponentBeginOverlap(CrossCollision)
  (params (OverlappedComponent :type Primitive%20Component%20Object%20Reference) (OtherActor :type Actor%20Object%20Reference) (OtherComp :type Primitive%20Component%20Object%20Reference) (OtherBodyIndex :type Integer) (bFromSweep :type Boolean) (SweepResult :type Hit%20Result%20Structure%20%28by%20ref%29))
  (if (Variables|Default|GetIsArmed)
    (Utilities|Casting|CastToBP_FirstPersonCharacter OtherActor)
    (Utilities|FlowControl|DoOnce false
      (:Completed
        (bind _turn (Timeline|RotationAnimation PlayFromStart)
          (:Update
            (Transformation|SetRelativeRotation (Variables|Default|Getcross) (Math|Rotator|CombineRotators (Variables|Default|GetInitialRotation) (Math|Rotator|MakeRotator 0.0 (Math|Float|Lerp 0.0 (Variables|Default|GetTargetRotationAngle) _turn) 0.0)) false false)))))))

(event EventBeginPlay
  (Variables|Default|SetInitialRotation (Variables|/Script/Engine.SceneComponent|GetRelativeRotation (Variables|Default|Getcross))))

(event Collision|EventActorBeginOverlap
  (params (OtherActor :type Actor%20Object%20Reference)))

(event EventTick
  (params (DeltaSeconds :type Float%20%28single-precision%29)))

(event EventActiveAnomaly
  (Variables|Default|SetIsArmed true))

(event EventResetAnomaly
  (Utilities|FlowControl|Sequence
    (:then_0
      (bind _turn (Timeline|RotationAnimation Stop)
        (:Update
          (Transformation|SetRelativeRotation (Variables|Default|Getcross) (Math|Rotator|CombineRotators (Variables|Default|GetInitialRotation) (Math|Rotator|MakeRotator 0.0 (Math|Float|Lerp 0.0 (Variables|Default|GetTargetRotationAngle) _turn) 0.0)) false false))))
    (:then_1
      (Transformation|SetRelativeRotation (Variables|Default|Getcross) (Variables|Default|GetInitialRotation) false false)
      (Variables|Default|SetIsArmed false))
    (:then_2
      (Utilities|FlowControl|DoOnce false) ; enters at Reset
    )))

(fn ConstructionScript)