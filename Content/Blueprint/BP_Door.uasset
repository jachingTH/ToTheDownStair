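; BP_Door is an interactable door that swings open or closed each time OnInteract fires.
; BeginPlay stores the door component's relative rotation as the closed pose.
; OnInteract plays the DoorAnimation timeline forward or in reverse, lerping between closed and open rotations, then flips the open state when finished.
; IsCurrentlyAnimating exposes the in-motion flag, which OnInteract sets but does not check itself.
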(event EventBeginPlay
  (Variables|Default|SetDoorCloseRotation (Variables|/Script/Engine.SceneComponent|GetRelativeRotation (Variables|Default|GetDoor-Pack-Free_Door-01))))

(event Collision|EventActorBeginOverlap
  (params (OtherActor :type Actor%20Object%20Reference)))

(event EventTick
  (params (DeltaSeconds :type Float%20%28single-precision%29)))

(event EventOnInteract
  (Variables|Default|SetIsAnimating true)
  (if (Variables|Default|GetIsDoorOpen)
    (bind _alpha (Timeline|DoorAnimation ReverseFromEnd)
      (:Update
        (Transformation|SetRelativeRotation (Variables|Default|GetDoor-Pack-Free_Door-01) (Math|Rotator|Lerp(Rotator) (Variables|Default|GetDoorCloseRotation) (Variables|Default|GetDoorOpenRotation) _alpha) false false))
      (:Finished
        (Variables|Default|SetIsAnimating false)
        (Variables|Default|SetIsDoorOpen (not (Variables|Default|GetIsDoorOpen)))))
    (else
      (Timeline|DoorAnimation PlayFromStart))))

(fn ConstructionScript)

(fn IsCurrentlyAnimating
  (return (Variables|Default|GetIsAnimating)))