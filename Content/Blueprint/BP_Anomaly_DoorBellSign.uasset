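; BP_Anomaly_DoorBellSign is an anomaly actor that shows or hides decals as it is activated or reset.
; ActiveAnomaly and ResetAnomaly set IsArmed, print debug text and call UpdateDecalVisibility, which also runs on BeginPlay.
; That function affects every DecalActor in the level, creating a dynamic material instance on each call and setting its VisibleAlpha parameter from IsArmed.
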(event EventBeginPlay
  (Development|PrintString "데칼 작용!" true true "(R=0.000000,G=0.660000,B=1.000000,A=1.000000)" 5.0)
  (CallFunction|UpdateDecalVisibility))

(event Collision|EventActorBeginOverlap
  (params (OtherActor :type Actor%20Object%20Reference)))

(event EventTick
  (params (DeltaSeconds :type Float%20%28single-precision%29)))

(event EventActiveAnomaly
  (Variables|Default|SetIsArmed true)
  (Development|PrintString "Armed Changed!" true true "(R=0.000000,G=0.660000,B=1.000000,A=1.000000)" 5.0)
  (CallFunction|UpdateDecalVisibility))

(event EventResetAnomaly
  (Variables|Default|SetIsArmed false)
  (Development|PrintString "Armed Changed!" true true "(R=0.000000,G=0.660000,B=1.000000,A=1.000000)" 5.0)
  (CallFunction|UpdateDecalVisibility))

(fn ConstructionScript)

(fn UpdateDecalVisibility
  (bind _outactors (Actor|GetAllActorsOfClass "/Script/Engine.DecalActor"))
  (for _array_element _outactors
    (bind _returnvalue (Rendering|Material|CreateDynamicMaterialInstance (Actor|GetComponentbyClass _array_element "/Script/Engine.DecalComponent") :!class /Script/Engine.DecalComponent))
    (Rendering|Material|SetScalarParameterValue _returnvalue "VisibleAlpha" (Math|Float|SelectFloat 1.0 0.0 (Variables|Default|GetIsArmed)) :!class /Script/Engine.MaterialInstanceDynamic)))